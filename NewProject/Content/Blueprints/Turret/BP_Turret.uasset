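; Auto-turret that scans for the first-person player character and fires bullets at it.
; Each Tick a forward line trace sets or, after a short delay, clears the target; the turret yaws steadily while searching and interpolates toward the target when locked.
; A looping fire-rate timer spawns bullets from alternating barrels while locked, randomly scaling the turret's rotation for inaccuracy.
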(event `self.ReceiveBeginPlay`
  ; OnLevelStart
  (set `self.ReadyToShoot` true)
  (`|ExecutionSequence`
    (:`then_0`
      (set `self.RayDistance` 1500.0))
    (:`then_1`
      (set `self.RotateSpeed` 25.0))
    (:`then_2`
      (bind _output_get (set `self.FireRate` 0.2)))
    (:`then_3`
      (set `self.AccuracyMod` 1.5))
    (:`then_4`
      (set `self.MaxRotateSpeed` 1500.0))
    (:`then_5`
      (`KismetSystemLibrary.K2_SetTimerDelegate` (delegate `ResetReadyToShoot`) _output_get true))))

(event `self.ReceiveTick`
  (params (DeltaSeconds :type "Float (single-precision)"))
  (bind _returnvalue (`self.K2_GetActorLocation`))
  (bind _turret (`self.Turret`))
  (bind _returnvalue_2 (`SceneComponent.K2_GetComponentLocation` _turret))
  ; Update with 2 Sequences one constantly casting the ray one to rotate the tturret if locked on
  (`|ExecutionSequence`
    (:`then_0`
      ; Ray trace only resulting from hitting actors
      (bind _outhit (`KismetSystemLibrary.LineTraceSingle` :`Start` _returnvalue_2 :`End` (+ _returnvalue_2 (* (`KismetMathLibrary.GetForwardVector` (`SceneComponent.K2_GetComponentRotation` _turret)) (`self.RayDistance`))) :`TraceChannel` "TraceTypeQuery1" :`DrawDebugType` "ForOneFrame"))
      ; Cast Logic to see if actor is theBPFP Character specifically locking or unlocking, setting or clearing target if LOS is broken or not
      (bind _asbp_fpcharacter (cast `/Game/Blueprints/Character/BP_FPCharacter` (`.HitActor` (`GameplayStatics.BreakHitResult` _outhit)))
        (:`then`
          (set `self.ShouldShoot` true)
          (set `self.LockedOn` true)
          (set `self.Target` _asbp_fpcharacter))
        (:`CastFailed`
          (`KismetSystemLibrary.Delay` 0.2)
          (set `self.ShouldShoot` false)
          (if (not (`self.ShouldShoot`))
            (if (`self.LockedOn`)
              _
              (else
                _))
            (set `self.Target` null)
            (set `self.LockedOn` false)))))
    (:`then_1`
      ; AutoRotate to search for player
      (if (`self.LockedOn`)
        ; Rotate if locked on
        (`self.K2_SetActorTransform` (`KismetMathLibrary.MakeTransform` _returnvalue (`KismetMathLibrary.RInterpTo` (`self.K2_GetActorRotation`) (`KismetMathLibrary.FindLookAtRotation` _returnvalue (`self.K2_GetActorLocation` (`self.Target`))) (`GameplayStatics.GetWorldDeltaSeconds`) (`self.MaxRotateSpeed`))))
        (else
          (`self.K2_SetActorTransform` (`KismetMathLibrary.MakeTransform` (`self.K2_GetActorLocation`) (`KismetMathLibrary.MakeRotator` 0.0 0.0 (+ (* DeltaSeconds (`self.RotateSpeed`)) (.yaw (`self.K2_GetActorRotation`)))))))))))

(event `ResetReadyToShoot`
  ; Event to check if the turret should shoot, if its locked onto the player, and to alternate between barrells
  (if (`self.LockedOn`)
    (if (`self.ShouldShoot`)
      (if (`self.Alternate`)
        ; Spawns according to which barrell
        (`|SpawnActorFromClass` "/Game/Blueprints/Turret/BP_TurretBullet.BP_TurretBullet_C" (`KismetMathLibrary.MakeTransform` (`SceneComponent.K2_GetComponentLocation` (`self.BarrelEnd2`)) (* (`SceneComponent.K2_GetComponentRotation` (`self.Turret`)) (`KismetMathLibrary.RandomFloatInRange` 0.1 (`self.AccuracyMod`)))) "Undefined" "MultiplyWithRoot" null null)
        (else
          (`|SpawnActorFromClass` "/Game/Blueprints/Turret/BP_TurretBullet.BP_TurretBullet_C" (`KismetMathLibrary.MakeTransform` (`SceneComponent.K2_GetComponentLocation` (`self.BarrelEnd`)) (* (`SceneComponent.K2_GetComponentRotation` (`self.Turret`)) (`KismetMathLibrary.RandomFloatInRange` 0.1 (`self.AccuracyMod`)))) "Undefined" "MultiplyWithRoot" null null)))
      ; Disable ReadyToShoot to simulate fire rate and equate Alternate variable to opposite
      (set `self.ReadyToShoot` false)
      (set `self.Alternate` (not (`self.Alternate`))))))

(fn `UserConstructionScript`)